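; BP_Tunnel is one segment of an endless tunnel, with a rotating wall that damages BP_Player on overlap.
; RandomizeWall picks one of four hole meshes, gives it a random roll, and spawns either a health pack or, more often, an enemy near the wall.
; When the player enters TriggerZone, it adds score, has TunnelSpawner spawn another tunnel, then destroys itself and any spawned pickup or enemy.
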(event `self.ReceiveTick`
  (params (DeltaSeconds :type "Float (single-precision)"))
  (`SceneComponent.K2_AddLocalRotation` (`self.WallMesh`) (`KismetMathLibrary.MakeRotator` (* DeltaSeconds (`self.RotateSpeed`))) false false))

(event `self.TriggerZone.OnComponentBeginOverlap`
  (params (OverlappedComponent :type "PrimitiveComponent Object Reference") (OtherActor :type "Actor Object Reference") (OtherComp :type "PrimitiveComponent Object Reference") (OtherBodyIndex :type Integer) (bFromSweep :type Boolean) (SweepResult :type "HitResult Structure (by ref)"))
  (bind _healthpack (`self.HealthPack`))
  (bind _enemy (`self.Enemy`))
  (bind _asbp_player (cast `/Game/InfiniteMatrix/Blueprints/BP_Player` OtherActor))
  (`/Engine/EditorBlueprintResources/StandardMacros.IncrementInt` (`/Game/InfiniteMatrix/Blueprints/BP_Player.Score` _asbp_player)
    (:`  `
      (`/Game/InfiniteMatrix/Blueprints/BP_TunnelSpawner.SpawnTunnelAtSpawnPoint` (`self.TunnelSpawner`))
      (`|ExecutionSequence`
        (:`then_0`
          (`/Engine/EditorBlueprintResources/StandardMacros.IsValid` _healthpack
            (:`Is Valid`
              (`self.K2_DestroyActor` _healthpack))))
        (:`then_1`
          (`/Engine/EditorBlueprintResources/StandardMacros.IsValid` _enemy
            (:`Is Valid`
              (`self.K2_DestroyActor` _enemy))))
        (:`then_2`
          (`self.K2_DestroyActor`))))))

(event `self.WallMesh.OnComponentBeginOverlap`
  (params (OverlappedComponent :type "PrimitiveComponent Object Reference") (OtherActor :type "Actor Object Reference") (OtherComp :type "PrimitiveComponent Object Reference") (OtherBodyIndex :type Integer) (bFromSweep :type Boolean) (SweepResult :type "HitResult Structure (by ref)"))
  (bind _asbp_player (cast `/Game/InfiniteMatrix/Blueprints/BP_Player` OtherActor))
  (`/Game/InfiniteMatrix/Blueprints/BP_Player.DecreaseHealth` _asbp_player))

(fn `RandomizeWall`
  (bind _wallmesh (`self.WallMesh`))
  (`StaticMeshComponent.SetStaticMesh` _wallmesh (select `int` (`KismetMathLibrary.RandomIntegerInRange` 0 3) :`0` "/Game/InfiniteMatrix/Meshes/SM_Hole_01.SM_Hole_01" :`1` "/Game/InfiniteMatrix/Meshes/SM_Hole_02.SM_Hole_02" :`2` "/Game/InfiniteMatrix/Meshes/SM_Hole_03.SM_Hole_03" :`3` "/Game/InfiniteMatrix/Meshes/SM_Hole_04.SM_Hole_04" :!type "StaticMesh Object Reference"))
  (`SceneComponent.K2_AddLocalRotation` _wallmesh (`KismetMathLibrary.MakeRotator` (`KismetMathLibrary.RandomFloatInRange` 0.0 360.0)) false false)
  (if (== (`KismetMathLibrary.RandomIntegerInRange` 0 3) 0)
    (`self.SpawnHealthPack`)
    (else
      (`self.SpawnEnemy`))))

(fn `SpawnEnemy`
  (bind (_returnvalue_x _returnvalue_y _returnvalue_z) (`KismetMathLibrary.BreakVector` (`SceneComponent.K2_GetComponentLocation` (`self.WallMesh`))))
  (bind _returnvalue (`|SpawnActorFromClass` "/Game/InfiniteMatrix/Blueprints/BP_Enemy.BP_Enemy_C" (`KismetMathLibrary.MakeTransform` (`KismetMathLibrary.MakeVector` (+ (`KismetMathLibrary.RandomFloatInRange` -400.0 -100.0) _returnvalue_x) (+ _returnvalue_y (`KismetMathLibrary.RandomFloatInRange` -200.0 200.0)) (+ _returnvalue_z (`KismetMathLibrary.RandomFloatInRange` -200.0 200.0))) (struct :`Yaw` 90.0)) "Undefined" "OverrideRootScale" null null))
  (set `self.Enemy` _returnvalue))

(fn `SpawnHealthPack`
  (bind (_returnvalue_x _returnvalue_y _returnvalue_z) (`KismetMathLibrary.BreakVector` (`SceneComponent.K2_GetComponentLocation` (`self.WallMesh`))))
  (bind _returnvalue (`|SpawnActorFromClass` "/Game/InfiniteMatrix/Blueprints/BP_HealthPack.BP_HealthPack_C" (`KismetMathLibrary.MakeTransform` (`KismetMathLibrary.MakeVector` (+ (`KismetMathLibrary.RandomFloatInRange` -400.0 -100.0) _returnvalue_x) (+ _returnvalue_y (`KismetMathLibrary.RandomFloatInRange` -200.0 200.0)) (+ _returnvalue_z (`KismetMathLibrary.RandomFloatInRange` -200.0 200.0))) (struct) (0.5 0.5 0.5)) "Undefined" "OverrideRootScale" null null))
  (set `self.HealthPack` _returnvalue))

(fn `UserConstructionScript`)