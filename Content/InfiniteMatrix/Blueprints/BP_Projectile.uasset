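; BP_Projectile is a projectile actor that travels in a straight line and removes itself from the world.
; Each Tick moves it along world X at ForwardSpeed with a swept offset and counts TimeAlive down, destroying it when time runs out.
; It is also destroyed when its Cylinder component ends an overlap, rather than begins one, with any component lacking the "Clear" tag.
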(event `self.ReceiveTick`
  (params (DeltaSeconds :type "Float (single-precision)"))
  (bind _returnvalue (- (`self.TimeAlive`) DeltaSeconds))
  (`self.K2_AddActorWorldOffset` (`KismetMathLibrary.MakeVector` (* DeltaSeconds (`self.ForwardSpeed`))) true)
  (if (<= _returnvalue 0.0)
    (`self.K2_DestroyActor`)
    (else
      (set `self.TimeAlive` _returnvalue))))

(event `self.Cylinder.OnComponentEndOverlap`
  (params (OverlappedComponent :type "PrimitiveComponent Object Reference") (OtherActor :type "Actor Object Reference") (OtherComp :type "PrimitiveComponent Object Reference") (OtherBodyIndex :type Integer))
  (if (not (`ActorComponent.ComponentHasTag` OtherComp "Clear"))
    (`self.K2_DestroyActor`)))

(fn `UserConstructionScript`)